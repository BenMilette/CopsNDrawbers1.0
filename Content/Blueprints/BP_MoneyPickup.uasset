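; BP_MoneyPickup is an AI-driven money pickup that runs BT_Money and adds its value to the player's score.
; On spawn it takes the first Values entry, shown as dollar text that rotates every tick.
; A player capsule overlap awards score and plays a sound, while police capsules consume it without scoring.
; Either way, MyGameMode spawns a replacement and decrements its pickup count before the actor is destroyed.
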(event OnComponentBeginOverlap(CapsuleComponent)
  (params (OverlappedComponent :type Primitive%20Component%20Object%20Reference) (OtherActor :type Actor%20Object%20Reference) (OtherComp :type Primitive%20Component%20Object%20Reference) (OtherBodyIndex :type Integer) (bFromSweep :type Boolean) (SweepResult :type Hit%20Result%20Structure%20%28by%20ref%29))
  (bind _asbp_player_character (Utilities|Casting|CastToBP_PlayerCharacter OtherActor)
    (:then
      (Variables|/Game/Blueprints/BP_PlayerCharacter.BP_PlayerCharacter_C|SetScore _asbp_player_character (+ (Variables|Default|GetValue) (Variables|/Game/Blueprints/BP_PlayerCharacter.BP_PlayerCharacter_C|GetScore _asbp_player_character)))
      (Audio|PlaySound2D "/Game/Assets/SFX/money_pickup_Cue.money_pickup_Cue" 1.0 1.0 0.0 0 0))
    (:CastFailed
      (Utilities|Casting|CastToBP_Police OtherActor)
      (Utilities|Casting|CastToCapsuleComponent OtherComp)))
  (bind _asmy_game_mode (Utilities|Casting|CastToMyGameMode (Game|GetGameMode)))
  (Default|SpawnMoneyPickup _asmy_game_mode)
  (Variables|/Game/Blueprints/MyGameMode.MyGameMode_C|SetAmountMoneyPickups _asmy_game_mode (- (Variables|/Game/Blueprints/MyGameMode.MyGameMode_C|GetAmountMoneyPickups _asmy_game_mode) 1))
  (Actor|DestroyActor))

(event EventBeginPlay
  (AI|RunBehaviorTree (AI|GetAIController self) "/Game/AI/BT_Money.BT_Money")
  (Variables|Default|SetValue (Utilities|Array|Get(acopy) (Variables|Default|GetValues) (Math|Random|RandomIntegerinRange 0 0)))
  (Rendering|Components|TextRender|SetText (Variables|Default|GetTextRender) (Utilities|Text|FormatText "${Value}" (Variables|Default|GetValue))))

(event Collision|EventActorBeginOverlap
  (params (OtherActor :type Actor%20Object%20Reference)))

(event EventTick
  (params (DeltaSeconds :type Float%20%28single-precision%29))
  (bind _textrender (Variables|Default|GetTextRender))
  (Transformation|SetWorldRotation _textrender (Math|Rotator|CombineRotators (Transformation|GetWorldRotation _textrender) "0,1.000000, 0") false false))

(fn ConstructionScript)