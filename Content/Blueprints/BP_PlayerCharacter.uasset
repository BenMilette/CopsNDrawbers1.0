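; Player car character that follows a path drawn by pressing and dragging from its mesh, and ends the game when hit by police.
; While held, Tick projects the mouse onto the Z=0 plane, adds spaced points to BPSpline and rebuilds spline meshes with time-driven materials.
; Release plays a length-scaled timeline moving the car along the spline at constant speed, with engine sounds.
; CancelPath turns the path red and aborts the move.
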(event OnComponentHit(CapsuleComponent)
  (params (HitComponent :type Primitive%20Component%20Object%20Reference) (OtherActor :type Actor%20Object%20Reference) (OtherComp :type Primitive%20Component%20Object%20Reference) (NormalImpulse :type Vector :default "0, 0, 0") (Hit :type Hit%20Result%20Structure%20%28by%20ref%29))
  (Utilities|Casting|CastToBP_Police OtherActor)
  (Utilities|Casting|CastToCapsuleComponent OtherComp)
  (Utilities|FlowControl|DoOnce false
    (:Completed
      (CallFunction|GameOver))))

(event OnClicked(Mesh)
  (params (TouchedComponent :type Primitive%20Component%20Object%20Reference) (ButtonPressed :type Key%20Structure))
  (bind _pathmeshes (Variables|Default|GetPathMeshes))
  (bind _bpspline (Variables|Default|GetBPSpline))
  (bind _spline (Variables|/Game/Blueprints/BP_Spline.BP_Spline_C|GetSpline _bpspline))
  (Utilities|FlowControl|Sequence
    (:then_0
      (Utilities|IsValid (Variables|Default|GetSoundVar)
        (:Is%20Valid
          (Audio|Components|Audio|Stop (Variables|Default|GetSoundVar)))
        (:Is%20Not%20Valid
          _))
      (bind _returnvalue (Audio|SpawnSound2D "/Game/Assets/SFX/car_start_idle_Cue.car_start_idle_Cue" 1.0 1.0 0.0 0))
      (Variables|Default|SetSoundVar _returnvalue))
    (:then_1
      (Utilities|FlowControl|Sequence
        (:then_0
          (bind _animationalpha (Timeline|PathTimeLine Stop)
            (:Update
              (Transformation|SetActorTransform (Math|Transform|MakeTransform (Math|Vector|MakeVector (.x (Spline|GetLocationatDistanceAlongSpline _spline (* _animationalpha (Spline|GetSplineLength _spline)) "World")) (.y (Spline|GetLocationatDistanceAlongSpline _spline (* _animationalpha (Spline|GetSplineLength _spline)) "World")) (.z (Transformation|GetActorLocation))) (Spline|GetRotationatDistanceAlongSpline _spline (* _animationalpha (Spline|GetSplineLength _spline)) "World"))))
            (:Finished
              (for (_array_element _array_index) _pathmeshes
                (Utilities|IsValid _array_element
                  (:Is%20Valid
                    (Components|DestroyComponent _array_element)
                    (if (== _array_index (- (Utilities|Array|Length _pathmeshes) 2))
                      (Utilities|IsValid (Variables|Default|GetSoundVar)
                        (:Is%20Valid
                          (Audio|Components|Audio|Stop (Variables|Default|GetSoundVar)))
                        (:Is%20Not%20Valid
                          _))
                      (bind _returnvalue_2 (Audio|SpawnSound2D "/Game/Assets/SFX/car_stop_Cue.car_stop_Cue" 0.25 1.25 0.5 0))
                      (Variables|Default|SetSoundVar _returnvalue_2)))))
              (Transformation|SetActorLocation (Variables|Default|GetBPSpline) (Transformation|GetActorLocation) false false))))
        (:then_1
          (CallFunction|EmptySpline)
          (bind _position (CallFunction|GetMousePosition))
          (Spline|AddSplinePoint (Variables|/Game/Blueprints/BP_Spline.BP_Spline_C|GetSpline (Variables|Default|GetBPSpline)) _position "World" true)
          (Variables|Default|SetSplineIndex (+ (Variables|Default|GetSplineIndex) 1))
          (Variables|Default|SetLeftClickPressed true))
        (:then_2
          (Variables|Default|SetGame%20Time 0.0))))))

(event OnInputTouchBegin(Mesh)
  (params (FingerIndex :type ETouchIndex%20Enum :default "Touch1") (TouchedComponent :type Primitive%20Component%20Object%20Reference))
  (bind _pathmeshes (Variables|Default|GetPathMeshes))
  (bind _bpspline (Variables|Default|GetBPSpline))
  (bind _spline (Variables|/Game/Blueprints/BP_Spline.BP_Spline_C|GetSpline _bpspline))
  (Utilities|FlowControl|Sequence
    (:then_0
      (Utilities|IsValid (Variables|Default|GetSoundVar)
        (:Is%20Valid
          (Audio|Components|Audio|Stop (Variables|Default|GetSoundVar)))
        (:Is%20Not%20Valid
          _))
      (bind _returnvalue (Audio|SpawnSound2D "/Game/Assets/SFX/car_start_idle_Cue.car_start_idle_Cue" 1.0 1.0 0.0 0))
      (Variables|Default|SetSoundVar _returnvalue))
    (:then_1
      (Utilities|FlowControl|Sequence
        (:then_0
          (bind _animationalpha (Timeline|PathTimeLine Stop)
            (:Update
              (Transformation|SetActorTransform (Math|Transform|MakeTransform (Math|Vector|MakeVector (.x (Spline|GetLocationatDistanceAlongSpline _spline (* _animationalpha (Spline|GetSplineLength _spline)) "World")) (.y (Spline|GetLocationatDistanceAlongSpline _spline (* _animationalpha (Spline|GetSplineLength _spline)) "World")) (.z (Transformation|GetActorLocation))) (Spline|GetRotationatDistanceAlongSpline _spline (* _animationalpha (Spline|GetSplineLength _spline)) "World"))))
            (:Finished
              (for (_array_element _array_index) _pathmeshes
                (Utilities|IsValid _array_element
                  (:Is%20Valid
                    (Components|DestroyComponent _array_element)
                    (if (== _array_index (- (Utilities|Array|Length _pathmeshes) 2))
                      (Utilities|IsValid (Variables|Default|GetSoundVar)
                        (:Is%20Valid
                          (Audio|Components|Audio|Stop (Variables|Default|GetSoundVar)))
                        (:Is%20Not%20Valid
                          _))
                      (bind _returnvalue_2 (Audio|SpawnSound2D "/Game/Assets/SFX/car_stop_Cue.car_stop_Cue" 0.25 1.25 0.5 0))
                      (Variables|Default|SetSoundVar _returnvalue_2)))))
              (Transformation|SetActorLocation (Variables|Default|GetBPSpline) (Transformation|GetActorLocation) false false))))
        (:then_1
          (CallFunction|EmptySpline)
          (bind _position (CallFunction|GetMousePosition))
          (Spline|AddSplinePoint (Variables|/Game/Blueprints/BP_Spline.BP_Spline_C|GetSpline (Variables|Default|GetBPSpline)) _position "World" true)
          (Variables|Default|SetSplineIndex (+ (Variables|Default|GetSplineIndex) 1))
          (Variables|Default|SetLeftClickPressed true))
        (:then_2
          (Variables|Default|SetGame%20Time 0.0))))))

(event OnInputTouchEnd(Mesh)
  (params (FingerIndex :type ETouchIndex%20Enum :default "Touch1") (TouchedComponent :type Primitive%20Component%20Object%20Reference))
  (bind _pathmeshes (Variables|Default|GetPathMeshes))
  (bind _bpspline (Variables|Default|GetBPSpline))
  (bind _spline (Variables|/Game/Blueprints/BP_Spline.BP_Spline_C|GetSpline _bpspline))
  (if (Variables|Default|GetLeftClickPressed)
    (if (Variables|Default|GetCancelPath)
      (for _array_element (Variables|Default|GetPathMeshes)
        (Components|DestroyComponent _array_element))
      (else
        (Utilities|FlowControl|Sequence
          (:then_0
            (Utilities|IsValid (Variables|Default|GetSoundVar)
              (:Is%20Valid
                (Audio|Components|Audio|Stop (Variables|Default|GetSoundVar)))
              (:Is%20Not%20Valid
                _))
            (bind _returnvalue (Audio|SpawnSound2D "/Game/Assets/SFX/car_driving_Cue.car_driving_Cue" 1.0 1.0 0.0 0))
            (Variables|Default|SetSoundVar _returnvalue))
          (:then_1
            (Variables|Default|SetLeftClickPressed false)
            (Components|Timeline|SetPlayRate (Variables|Default|GetPathTimeLine) (* (/ 1.0 (Spline|GetSplineLength (Variables|/Game/Blueprints/BP_Spline.BP_Spline_C|GetSpline (Variables|Default|GetBPSpline)))) (Variables|Default|GetSpeed)))
            (bind _animationalpha (Timeline|PathTimeLine PlayFromStart)
              (:Update
                (Transformation|SetActorTransform (Math|Transform|MakeTransform (Math|Vector|MakeVector (.x (Spline|GetLocationatDistanceAlongSpline _spline (* _animationalpha (Spline|GetSplineLength _spline)) "World")) (.y (Spline|GetLocationatDistanceAlongSpline _spline (* _animationalpha (Spline|GetSplineLength _spline)) "World")) (.z (Transformation|GetActorLocation))) (Spline|GetRotationatDistanceAlongSpline _spline (* _animationalpha (Spline|GetSplineLength _spline)) "World"))))
              (:Finished
                (for (_array_element_2 _array_index) _pathmeshes
                  (Utilities|IsValid _array_element_2
                    (:Is%20Valid
                      (Components|DestroyComponent _array_element_2)
                      (if (== _array_index (- (Utilities|Array|Length _pathmeshes) 2))
                        (Utilities|IsValid (Variables|Default|GetSoundVar)
                          (:Is%20Valid
                            (Audio|Components|Audio|Stop (Variables|Default|GetSoundVar)))
                          (:Is%20Not%20Valid
                            _))
                        (bind _returnvalue_2 (Audio|SpawnSound2D "/Game/Assets/SFX/car_stop_Cue.car_stop_Cue" 0.25 1.25 0.5 0))
                        (Variables|Default|SetSoundVar _returnvalue_2)))))
                (Transformation|SetActorLocation (Variables|Default|GetBPSpline) (Transformation|GetActorLocation) false false)))))))))

(event EventBeginPlay
  (Transformation|SetActorLocation (Variables|Default|GetBPSpline) (Transformation|GetActorLocation) false false))

(event EventTick
  (params (DeltaSeconds :type Float%20%28single-precision%29))
  (if (Variables|Default|GetLeftClickPressed)
    (Variables|Default|SetGame%20Time (+ DeltaSeconds (Variables|Default|GetGame%20Time)))
    (if (Variables|Default|GetCancelPath)
      (CallFunction|DrawPath)
      (Variables|Default|SetLeftClickPressed false)
      (else
        (bind _add_spline_point_ (CallFunction|CompareMousePosition))
        (if _add_spline_point_
          (bind _position (CallFunction|GetMousePosition))
          (Spline|AddSplinePoint (Variables|/Game/Blueprints/BP_Spline.BP_Spline_C|GetSpline (Variables|Default|GetBPSpline)) _position "World" true)
          (Variables|Default|SetSplineIndex (+ (Variables|Default|GetSplineIndex) 1))
          (CallFunction|DrawPath))))))

(event Input|MouseEvents|LeftMouseButton
  (params (Key :type Key%20Structure))
  (bind _pathmeshes (Variables|Default|GetPathMeshes))
  (bind _bpspline (Variables|Default|GetBPSpline))
  (bind _spline (Variables|/Game/Blueprints/BP_Spline.BP_Spline_C|GetSpline _bpspline))
  (:Released
    (if (Variables|Default|GetLeftClickPressed)
      (if (Variables|Default|GetCancelPath)
        (for _array_element (Variables|Default|GetPathMeshes)
          (Components|DestroyComponent _array_element))
        (else
          (Utilities|FlowControl|Sequence
            (:then_0
              (Utilities|IsValid (Variables|Default|GetSoundVar)
                (:Is%20Valid
                  (Audio|Components|Audio|Stop (Variables|Default|GetSoundVar)))
                (:Is%20Not%20Valid
                  _))
              (bind _returnvalue (Audio|SpawnSound2D "/Game/Assets/SFX/car_driving_Cue.car_driving_Cue" 1.0 1.0 0.0 0))
              (Variables|Default|SetSoundVar _returnvalue))
            (:then_1
              (Variables|Default|SetLeftClickPressed false)
              (Components|Timeline|SetPlayRate (Variables|Default|GetPathTimeLine) (* (/ 1.0 (Spline|GetSplineLength (Variables|/Game/Blueprints/BP_Spline.BP_Spline_C|GetSpline (Variables|Default|GetBPSpline)))) (Variables|Default|GetSpeed)))
              (bind _animationalpha (Timeline|PathTimeLine PlayFromStart)
                (:Update
                  (Transformation|SetActorTransform (Math|Transform|MakeTransform (Math|Vector|MakeVector (.x (Spline|GetLocationatDistanceAlongSpline _spline (* _animationalpha (Spline|GetSplineLength _spline)) "World")) (.y (Spline|GetLocationatDistanceAlongSpline _spline (* _animationalpha (Spline|GetSplineLength _spline)) "World")) (.z (Transformation|GetActorLocation))) (Spline|GetRotationatDistanceAlongSpline _spline (* _animationalpha (Spline|GetSplineLength _spline)) "World"))))
                (:Finished
                  (for (_array_element_2 _array_index) _pathmeshes
                    (Utilities|IsValid _array_element_2
                      (:Is%20Valid
                        (Components|DestroyComponent _array_element_2)
                        (if (== _array_index (- (Utilities|Array|Length _pathmeshes) 2))
                          (Utilities|IsValid (Variables|Default|GetSoundVar)
                            (:Is%20Valid
                              (Audio|Components|Audio|Stop (Variables|Default|GetSoundVar)))
                            (:Is%20Not%20Valid
                              _))
                          (bind _returnvalue_2 (Audio|SpawnSound2D "/Game/Assets/SFX/car_stop_Cue.car_stop_Cue" 0.25 1.25 0.5 0))
                          (Variables|Default|SetSoundVar _returnvalue_2)))))
                  (Transformation|SetActorLocation (Variables|Default|GetBPSpline) (Transformation|GetActorLocation) false false))))))))))

(fn ConstructionScript)

(fn GetMousePosition
  (bind _returnvalue (Game|GetPlayerController 0))
  (bind (_worldlocation _worlddirection) (Game|Player|ConvertMouseLocationToWorldSpace _returnvalue))
  (return (+ _worldlocation (* (* _worlddirection (/ (.Z (Math|Vector|BreakVector _worldlocation)) (.Z (Math|Vector|BreakVector _worlddirection)))) -1.0))))

(fn CompareMousePosition
  (bind _position (CallFunction|GetMousePosition))
  (return (>= (Math|Vector|VectorLength (- _position (Spline|GetLocationatSplinePoint (Variables|/Game/Blueprints/BP_Spline.BP_Spline_C|GetSpline (Variables|Default|GetBPSpline)) (Variables|Default|GetSplineIndex) "World"))) 25.0)))

(fn EmptySpline
  (Spline|ClearSplinePoints (Variables|/Game/Blueprints/BP_Spline.BP_Spline_C|GetSpline (Variables|Default|GetBPSpline)) true)
  (Variables|Default|SetSplineIndex 0))

(fn DrawPath
  (bind _bpspline (Variables|Default|GetBPSpline))
  (bind _bpspline_2 (Variables|Default|GetBPSpline))
  (bind _bpspline_3 (Variables|Default|GetBPSpline))
  (bind _spline (Variables|/Game/Blueprints/BP_Spline.BP_Spline_C|GetSpline _bpspline))
  (bind _spline_2 (Variables|/Game/Blueprints/BP_Spline.BP_Spline_C|GetSpline _bpspline_2))
  (bind _spline_3 (Variables|/Game/Blueprints/BP_Spline.BP_Spline_C|GetSpline _bpspline_3))
  (bind (_location _tangent) (Spline|GetLocationandTangentatSplinePoint _spline_2 0 "World"))
  (bind (_location_2 _tangent_2) (Spline|GetLocationandTangentatSplinePoint _spline_2 1 "World"))
  (bind _returnvalue (Spline|GetNumberOfSplinePoints _spline_3))
  (bind (_location_3 _tangent_3) (Spline|GetLocationandTangentatSplinePoint _spline_3 _returnvalue "World"))
  (bind _returnvalue_2 (- _returnvalue 2))
  (bind (_location_4 _tangent_4) (Spline|GetLocationandTangentatSplinePoint _spline_3 _returnvalue_2 "World"))
  (for _array_element (Variables|Default|GetPathMeshes)
    (Utilities|IsValid _array_element
      (:Is%20Valid
        (Components|DestroyComponent _array_element))))
  (Utilities|FlowControl|Sequence
    (:then_0
      (bind _returnvalue_3 (AddComponent|AddSplineMeshComponent true))
      (CallFunction|SetMaterial _returnvalue_3)
      (Utilities|Array|Add (Variables|Default|GetPathMeshes) _returnvalue_3)
      (if (Variables|Default|GetCancelPath)
        (CallFunction|ChangeMaterial _returnvalue_3))
      (SplineMesh|SetStartandEnd _returnvalue_3 _location _tangent _location_2 _tangent_2 true :!class /Script/Engine.SplineMeshComponent))
    (:then_1
      (for _index (range 1 (- (Spline|GetNumberOfSplinePoints (Variables|/Game/Blueprints/BP_Spline.BP_Spline_C|GetSpline (Variables|Default|GetBPSpline))) 3))
        (bind _returnvalue_4 (AddComponent|AddSplineMeshComponent true))
        (CallFunction|SetMaterial _returnvalue_4)
        (Utilities|Array|Add (Variables|Default|GetPathMeshes) _returnvalue_4)
        (if (Variables|Default|GetCancelPath)
          (CallFunction|ChangeMaterial _returnvalue_4))
        (SplineMesh|SetStartandEnd _returnvalue_4 (.Location (Spline|GetLocationandTangentatSplinePoint _spline _index "World")) (.Tangent (Spline|GetLocationandTangentatSplinePoint _spline _index "World")) (.Location (Spline|GetLocationandTangentatSplinePoint _spline (+ _index 1) "World")) (.Tangent (Spline|GetLocationandTangentatSplinePoint _spline (+ _index 1) "World")) true :!class /Script/Engine.SplineMeshComponent)))
    (:then_2
      (bind _returnvalue_5 (AddComponent|AddSplineMeshComponent true))
      (CallFunction|SetMaterial _returnvalue_5)
      (Utilities|Array|Add (Variables|Default|GetPathMeshes) _returnvalue_5)
      (if (Variables|Default|GetCancelPath)
        (CallFunction|ChangeMaterial _returnvalue_5))
      (SplineMesh|SetStartandEnd _returnvalue_5 _location_4 _tangent_4 _location_3 _tangent_3 true :!class /Script/Engine.SplineMeshComponent))))

(fn ChangeMaterial
  (params (Spline%20Point%20Mesh%20Component :type Mesh%20Component%20Object%20Reference))
  (Utilities|FlowControl|Sequence
    (:then_0
      (bind _returnvalue (Rendering|Material|CreateDynamicMaterialInstance Spline%20Point%20Mesh%20Component 0 "/Game/Materials/M_Path_Inst.M_Path_Inst" "None" :!class /Script/Engine.PrimitiveComponent))
      (Variables|Default|SetMaterial _returnvalue))
    (:then_1
      (Rendering|Material|SetVectorParameterValue (Variables|Default|GetMaterial) "Colour" "(R=1.000000,G=0.000000,B=0.000000,A=1.000000)" :!class /Script/Engine.MaterialInstanceDynamic)
      (Rendering|Material|SetVectorParameterValue (Variables|Default|GetMaterial) "Emissive Color" "(R=1.000000,G=0.500000,B=0.500000,A=1.000000)" :!class /Script/Engine.MaterialInstanceDynamic)
      (Rendering|Material|SetMaterial Spline%20Point%20Mesh%20Component 0 (Variables|Default|GetMaterial)))))

(fn GameOver
  (bind _returnvalue (UserInterface|CreateWidget "/Game/UI/Widget_GameOverMenu.Widget_GameOverMenu_C"))
  (bind _output_get (Variables|Default|SetGameOverWidget _returnvalue))
  (UserInterface|Viewport|AddtoViewport _output_get 0)
  (Game|SetGamePaused true))

(fn SetMaterial
  (params (Primitive%20Component :type Primitive%20Component%20Object%20Reference))
  (Utilities|FlowControl|Sequence
    (:then_0
      (bind _returnvalue (Rendering|Material|CreateDynamicMaterialInstance Primitive%20Component 0 "/Game/Materials/M_Path_Inst.M_Path_Inst" "Material" :!class /Script/Engine.PrimitiveComponent))
      (Variables|Default|SetMaterial _returnvalue))
    (:then_1
      (Rendering|Material|SetScalarParameterValue (Variables|Default|GetMaterial) "Time" (Variables|Default|GetGame%20Time) :!class /Script/Engine.MaterialInstanceDynamic))))