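; Game mode that spawns police and money pickups in every level except MainMenu.
; BeginPlay spawns one pickup, then one to three BP_Police on random "Ground"-tagged actors, scaled by the game instance's Difficulty.
; Tick accumulates a timer and uses a resettable DoOnce to add pickups at intervals while their count is below three.
; Pickup spawns set no location, as the random ground-location lookup is unused.
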(event EventBeginPlay
  (bind _returnvalue (Game|GetCurrentLevelName true))
  (if (not (Utilities|Enum|Equal(Enum) _returnvalue "MainMenu"))
    (CallFunction|SpawnMoneyPickup)
    (bind _asmy_game_instance (Utilities|Casting|CastToMyGameInstance (Game|GetGameInstance)))
    (switch Utilities|FlowControl|Switch|SwitchonEnum_Difficulty (Variables|/Game/Blueprints/MyGameInstance.MyGameInstance_C|GetDifficulty _asmy_game_instance)
      (:NewEnumerator0
        (CallFunction|SpawnPolice 1))
      (:NewEnumerator1
        (CallFunction|SpawnPolice 2))
      (:NewEnumerator2
        (CallFunction|SpawnPolice 3)))))

(event EventTick
  (params (DeltaSeconds :type Float%20%28single-precision%29))
  (bind _output_get (Variables|Default|SetSpawnMoneyTimer (+ DeltaSeconds (Variables|Default|GetSpawnMoneyTimer))))
  (if (== (Math|Integer|%(Integer) (Math|Float|Ceil _output_get) (Variables|Default|GetSpawnMoneyInterval)) 0)
    (Utilities|FlowControl|DoOnce false :!label _label
      (:Completed
        (if (< (Variables|Default|GetAmountMoneyPickups) 3)
          (CallFunction|SpawnMoneyPickup))))
    (else
      (goto _label Reset))))

(fn ConstructionScript)

(fn SpawnPolice
  (params (AmountToSpawn :type Integer))
  (bind _outactors (Actor|GetAllActorswithTag "Ground"))
  (for _index (range 0 (- AmountToSpawn 1))
    (Game|SpawnActorfromClass "/Game/Blueprints/BP_Police.BP_Police_C" (Math|Transform|MakeTransform (Transformation|GetActorLocation (Utilities|Array|Get(acopy) _outactors (Math|Random|RandomIntegerinRange 0 (Utilities|Array|LastIndex _outactors)))) "0, 0, 0" "1,1,1") "AlwaysSpawn" 0 0)))

(fn SpawnMoneyPickup
  (bind _outactors (Actor|GetAllActorswithTag "Ground"))
  (Game|SpawnActorfromClass "/Game/Blueprints/BP_MoneyPickup.BP_MoneyPickup_C" (Math|Transform|MakeTransform "0, 0, 0" "0, 0, 0" "1,1,1") "AlwaysSpawn" 0 0)
  (Variables|Default|SetAmountMoneyPickups (+ (Variables|Default|GetAmountMoneyPickups) 1)))