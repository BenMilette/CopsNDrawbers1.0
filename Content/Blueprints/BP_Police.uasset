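; Police AI character that runs BT_Cop and provides functions to patrol a looping list of targets or move to a chase position.
; Two vision cone overlaps flag the player or other police in view; spotting the player also drives emergency lights and a siren through a DoOnce.
; Leaving a cone starts a retriggerable delay before clearing player sight and lights.
; Capsule overlap with another police re-runs the behavior tree.
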(event OnComponentBeginOverlap(VisionCone1)
  (params (OverlappedComponent :type Primitive%20Component%20Object%20Reference) (OtherActor :type Actor%20Object%20Reference) (OtherComp :type Primitive%20Component%20Object%20Reference) (OtherBodyIndex :type Integer) (bFromSweep :type Boolean) (SweepResult :type Hit%20Result%20Structure%20%28by%20ref%29))
  (Utilities|FlowControl|Sequence
    (:then_0
      (Utilities|Casting|CastToBP_PlayerCharacter (stale OnComponentBeginOverlap(VisionCone2) OtherActor))
      (Variables|Default|SetPlayerInView true :!label _label)
      (Utilities|FlowControl|DoOnce false
        (:Completed
          (Rendering|Material|SetScalarParameterValue (Variables|Default|GetMaterialVar) "Lights" 1.0 :!class /Script/Engine.MaterialInstanceDynamic)
          (Utilities|IsValid (Variables|Default|GetSoundVar)
            (:Is%20Valid
              (Audio|Components|Audio|Stop (Variables|Default|GetSoundVar)))
            (:Is%20Not%20Valid
              (bind _returnvalue (Audio|SpawnSound2D "/Game/Assets/SFX/police_siren_Cue.police_siren_Cue" 1.0 1.0 0.0 0))
              (Variables|Default|SetSoundVar _returnvalue))))))
    (:then_1
      (Utilities|Casting|CastToBP_PlayerCharacter OtherActor)
      (goto _label))
    (:then_2
      (Utilities|Casting|CastToBP_Police (stale OnComponentBeginOverlap(VisionCone2) OtherActor))
      (Variables|Default|SetPoliceInView true :!label _label_2))
    (:then_3
      (Utilities|Casting|CastToBP_Police OtherActor)
      (goto _label_2))))

(event OnComponentEndOverlap(VisionCone1)
  (params (OverlappedComponent :type Primitive%20Component%20Object%20Reference) (OtherActor :type Actor%20Object%20Reference) (OtherComp :type Primitive%20Component%20Object%20Reference) (OtherBodyIndex :type Integer))
  (Utilities|Casting|CastToBP_PlayerCharacter OtherActor)
  (Utilities|FlowControl|RetriggerableDelay 3.0)
  (Rendering|Material|SetScalarParameterValue (Variables|Default|GetMaterialVar) "Lights" 0.0 :!class /Script/Engine.MaterialInstanceDynamic)
  (Variables|Default|SetPlayerInView false)
  (Utilities|IsValid (Variables|Default|GetSoundVar)
    (:Is%20Valid
      (Audio|Components|Audio|Stop (Variables|Default|GetSoundVar))
      (Utilities|FlowControl|DoOnce false) ; enters at Reset
    )))

(event OnComponentBeginOverlap(VisionCone2)
  (params (OverlappedComponent :type Primitive%20Component%20Object%20Reference) (OtherActor :type Actor%20Object%20Reference) (OtherComp :type Primitive%20Component%20Object%20Reference) (OtherBodyIndex :type Integer) (bFromSweep :type Boolean) (SweepResult :type Hit%20Result%20Structure%20%28by%20ref%29))
  (Utilities|FlowControl|Sequence
    (:then_0
      (Utilities|Casting|CastToBP_PlayerCharacter OtherActor)
      (Variables|Default|SetPlayerInView true :!label _label)
      (Utilities|FlowControl|DoOnce false
        (:Completed
          (Rendering|Material|SetScalarParameterValue (Variables|Default|GetMaterialVar) "Lights" 1.0 :!class /Script/Engine.MaterialInstanceDynamic)
          (Utilities|IsValid (Variables|Default|GetSoundVar)
            (:Is%20Valid
              (Audio|Components|Audio|Stop (Variables|Default|GetSoundVar)))
            (:Is%20Not%20Valid
              (bind _returnvalue (Audio|SpawnSound2D "/Game/Assets/SFX/police_siren_Cue.police_siren_Cue" 1.0 1.0 0.0 0))
              (Variables|Default|SetSoundVar _returnvalue))))))
    (:then_1
      (Utilities|Casting|CastToBP_PlayerCharacter (stale OnComponentBeginOverlap(VisionCone1) OtherActor))
      (goto _label))
    (:then_2
      (Utilities|Casting|CastToBP_Police OtherActor)
      (Variables|Default|SetPoliceInView true :!label _label_2))
    (:then_3
      (Utilities|Casting|CastToBP_Police (stale OnComponentBeginOverlap(VisionCone1) OtherActor))
      (goto _label_2))))

(event OnComponentEndOverlap(VisionCone2)
  (params (OverlappedComponent :type Primitive%20Component%20Object%20Reference) (OtherActor :type Actor%20Object%20Reference) (OtherComp :type Primitive%20Component%20Object%20Reference) (OtherBodyIndex :type Integer))
  (Utilities|Casting|CastToBP_PlayerCharacter OtherActor)
  (Utilities|FlowControl|RetriggerableDelay 3.0)
  (Rendering|Material|SetScalarParameterValue (Variables|Default|GetMaterialVar) "Lights" 0.0 :!class /Script/Engine.MaterialInstanceDynamic)
  (Variables|Default|SetPlayerInView false)
  (Utilities|IsValid (Variables|Default|GetSoundVar)
    (:Is%20Valid
      (Audio|Components|Audio|Stop (Variables|Default|GetSoundVar))
      (Utilities|FlowControl|DoOnce false) ; enters at Reset
    )))

(event OnComponentBeginOverlap(CapsuleComponent)
  (params (OverlappedComponent :type Primitive%20Component%20Object%20Reference) (OtherActor :type Actor%20Object%20Reference) (OtherComp :type Primitive%20Component%20Object%20Reference) (OtherBodyIndex :type Integer) (bFromSweep :type Boolean) (SweepResult :type Hit%20Result%20Structure%20%28by%20ref%29))
  (Utilities|Casting|CastToBP_Police OtherActor)
  (AI|RunBehaviorTree (AI|GetAIController self) "/Game/AI/BT_Cop.BT_Cop"))

(event EventBeginPlay
  (AI|RunBehaviorTree (AI|GetAIController self) "/Game/AI/BT_Cop.BT_Cop")
  (bind _returnvalue (Rendering|Material|CreateDynamicMaterialInstance (Variables|Character|GetMesh) 0 "/Game/Materials/M_Police.M_Police" "None" :!class /Script/Engine.PrimitiveComponent))
  (Variables|Default|SetMaterialVar _returnvalue))

(event EventTick
  (params (DeltaSeconds :type Float%20%28single-precision%29)))

(fn ConstructionScript)

(fn Patrol
  (bind _targets (Variables|Default|GetTargets))
  (AI|Navigation|SimpleMovetoLocation (Pawn|GetController) (Transformation|GetActorLocation (Utilities|Array|Get(acopy) _targets (Variables|Default|GetTargetIndex))))
  (if (<= (Math|Vector|VectorLength (- (Transformation|GetActorLocation) (Transformation|GetActorLocation (Utilities|Array|Get(acopy) _targets (Variables|Default|GetTargetIndex))))) 5e+01)
    (bind _output_get (Variables|Default|SetTargetIndex (+ (Variables|Default|GetTargetIndex) 1)))
    (if (> _output_get (Utilities|Array|LastIndex _targets))
      (Variables|Default|SetTargetIndex 0))))

(fn Chase
  (AI|Navigation|SimpleMovetoLocation (Pawn|GetController) (Variables|Default|GetChaseTargetPosition)))